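; BP_NPC1 is an NPC that cries out periodically, takes damage and dies.
; Any damage runs TakeDamage, which lowers clamped health and flags IsDead at zero.
; At zero health it plays a death sound, makes mesh and capsule static, then after a delay hides, disables mesh collision and destroys itself.
; A Delay on Tick throttles the cry to roughly every four seconds.
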(event `self.ReceiveAnyDamage`
  (params (Damage :type "Float (single-precision)") (DamageType :type "DamageType Object Reference") (InstigatedBy :type "Controller Object Reference") (DamageCauser :type "Actor Object Reference"))
  (bind _mesh (`self.Mesh`))
  ;[1 1 1] Daño y Muerte del NPC
  (`self.TakeDamage` Damage)
  (if (== (`self.VidaNPC`) 0.0)
    (`GameplayStatics.PlaySoundAtLocation` "/Game/Sounds/NPC1/MuerteNPC1.MuerteNPC1" (`self.K2_GetActorLocation`) (struct) 1.0 1.0 0.0 null null null)
    (`SceneComponent.SetMobility` (`self.Mesh`) "Static")
    (`SceneComponent.SetMobility` (`self.CapsuleComponent`) "Static")
    (`KismetSystemLibrary.Delay` 3.1)
    (`SceneComponent.SetVisibility` _mesh false false)
    (`PrimitiveComponent.SetCollisionEnabled` _mesh "NoCollision")
    (`self.K2_DestroyActor`)))

(event `self.ReceiveTick`
  (params (DeltaSeconds :type "Float (single-precision)"))
  ;[1 1 1] Sonido del NPC
  (`KismetSystemLibrary.Delay` 4.0)
  (`GameplayStatics.PlaySoundAtLocation` "/Game/Sounds/NPC1/GritoNPC1.GritoNPC1" (`self.K2_GetActorLocation`) (struct) 1.0 1.0 0.0 null null null))

(fn `TakeDamage`
  (params (Damage :type "Float (double-precision)"))
  (bind _output_get (set `self.VidaNPC` (`KismetMathLibrary.FClamp` (- (`self.VidaNPC`) Damage) 0.0 (`self.MaxVida`))))
  (if (== _output_get 0.0)
    (set `self.IsDead` true)))

(fn `UserConstructionScript`)