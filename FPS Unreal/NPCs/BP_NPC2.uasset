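; Enemy NPC for an FPS that chases the player on sight or sound and attacks on contact.
; PawnSensing events drive AI MoveTo, while Tick with a Delay repeats its cry.
; Capsule overlap with a PlayerController cast plays the attack sound, sets Ataque and subtracts from the player's Vidas after a delay.
; Damage lowers clamped health; at zero, it plays a death sound, turns static, then hides and destroys itself.
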(event `self.ReceiveTick`
  (params (DeltaSeconds :type "Float (single-precision)"))
  ;[1 1 1] Sonido NPC
  (`KismetSystemLibrary.Delay` 2.0)
  (`GameplayStatics.PlaySoundAtLocation` "/Game/Sounds/NPC2/NPC2Grito.NPC2Grito" (`self.K2_GetActorLocation`) (struct) 1.0 1.0 0.0 null null null))

(event `self.ReceiveAnyDamage`
  (params (Damage :type "Float (single-precision)") (DamageType :type "DamageType Object Reference") (InstigatedBy :type "Controller Object Reference") (DamageCauser :type "Actor Object Reference"))
  (bind _mesh (`self.Mesh`))
  ;[1 1 1] Daño y muerte NPC
  (`self.TakeDamage` Damage)
  (if (== (`self.VidaNPC`) 0.0)
    (`GameplayStatics.PlaySoundAtLocation` "/Game/Sounds/NPC2/MuerteNPC2.MuerteNPC2" (`self.K2_GetActorLocation`) (struct) 1.0 1.0 0.0 null null null)
    (`SceneComponent.SetMobility` (`self.Mesh`) "Static")
    (`SceneComponent.SetMobility` (`self.CapsuleComponent`) "Static")
    (`KismetSystemLibrary.Delay` 2.5)
    (`SceneComponent.SetVisibility` _mesh false false)
    (`PrimitiveComponent.SetCollisionEnabled` _mesh "NoCollision")
    (`self.K2_DestroyActor`)))

(event `self.PawnSensing.OnSeePawn`
  (params (Pawn :type "Pawn Object Reference"))
  ;[1 1 1] Escuchar y ver al jugador
  (`|AIMoveTo` self (0.0 0.0 0.0) Pawn 10.0))

(event `self.PawnSensing.OnHearNoise`
  (params (Instigator :type "Pawn Object Reference") (Location :type "Vector Structure (by ref)") (Volume :type "Float (single-precision)"))
  ;[1 1 1] Escuchar y ver al jugador
  (`|AIMoveTo` self (0.0 0.0 0.0) Instigator 10.0))

(event `self.CapsuleComponent.OnComponentBeginOverlap`
  (params (OverlappedComponent :type "PrimitiveComponent Object Reference") (OtherActor :type "Actor Object Reference") (OtherComp :type "PrimitiveComponent Object Reference") (OtherBodyIndex :type Integer) (bFromSweep :type Boolean) (SweepResult :type "HitResult Structure (by ref)"))
  ;[1 1 1] Daño al jugador
  (bind _asplayer_controller (cast `/Game/BluePrints/CharacterController/PlayerController` OtherActor))
  (`GameplayStatics.PlaySoundAtLocation` "/Game/Sounds/NPC2/AtaqueNPC2.AtaqueNPC2" (`self.K2_GetActorLocation`) (struct) 1.0 1.0 0.0 null null null)
  (set `self.Ataque` true)
  (`KismetSystemLibrary.Delay` 1.0)
  (set `/Game/BluePrints/CharacterController/PlayerController.Vidas` (- (`/Game/BluePrints/CharacterController/PlayerController.Vidas` _asplayer_controller) (`self.DañoAtaque`)) _asplayer_controller)
  (set `self.Ataque` false))

(fn `TakeDamage`
  (params (Damage :type "Float (double-precision)"))
  (bind _output_get (set `self.VidaNPC` (`KismetMathLibrary.FClamp` (- (`self.VidaNPC`) Damage) 0.0 (`self.MaxVidaNPC`))))
  (if (== _output_get 0.0)
    (set `self.IsDead` true)))

(fn `UserConstructionScript`)